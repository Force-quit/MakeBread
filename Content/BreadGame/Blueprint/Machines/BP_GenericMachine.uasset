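; Generic configurable production machine for the bread game that turns an input actor class into an output actor class.
; A matching input overlap toggles the input conveyor, destroys everything in the input collider, then spawns the output at the output collider after a delay.
; The output leaving toggles the conveyor again, and spawning bread notifies the game mode.
; The construction script applies the machine material to both meshes.
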(event `StartOutputProcess`
  ;[1 1 1] Spawning
  (for _array_element (`PrimitiveComponent.GetOverlappingActors` (`self.InputCollider`) null)
    (`self.K2_DestroyActor` _array_element))
  (`KismetSystemLibrary.Delay` (`self.processDelay`))
  (`|SpawnActorFromClass` (`self.OutputClass`) (`KismetMathLibrary.MakeTransform` (`SceneComponent.K2_GetComponentLocation` (`self.OutputCollider`))) "Undefined" "OverrideRootScale" null null)
  (if (== (`self.OutputClass`) "/Game/BreadGame/Blueprint/Breads/BP_Bread.BP_Bread_C")
    (bind _asbp_bread_game (cast `/Game/BreadGame/Blueprint/Game/GM_BreadGame` (`GameplayStatics.GetGameMode`)))
    (`/Game/BreadGame/Blueprint/Game/GM_BreadGame.OnBreadComplete` _asbp_bread_game)))

(event `self.InputCollider.OnComponentBeginOverlap`
  (params (OverlappedComponent :type "PrimitiveComponent Object Reference") (OtherActor :type "Actor Object Reference") (OtherComp :type "PrimitiveComponent Object Reference") (OtherBodyIndex :type Integer) (bFromSweep :type Boolean) (SweepResult :type "HitResult Structure (by ref)"))
  ;[1 1 1] Take input
  (if (== (`GameplayStatics.GetObjectClass` OtherActor) (`self.InputClass`))
    (`/Game/BreadGame/Blueprint/BP_Conveyer.SwitchState` (`self.InputConveyor`))
    (`self.StartOutputProcess`)))

(event `self.OutputCollider.OnComponentEndOverlap`
  (params (OverlappedComponent :type "PrimitiveComponent Object Reference") (OtherActor :type "Actor Object Reference") (OtherComp :type "PrimitiveComponent Object Reference") (OtherBodyIndex :type Integer))
  ;[1 1 1] Output left machine
  (if (== (`GameplayStatics.GetObjectClass` OtherActor) (`self.OutputClass`))
    (`/Game/BreadGame/Blueprint/BP_Conveyer.SwitchState` (`self.InputConveyor`))))

(fn `UserConstructionScript`
  (`PrimitiveComponent.SetMaterial` (`self.Small`) 0 (`self.machineMaterial`))
  (`PrimitiveComponent.SetMaterial` (`self.Big`) 0 (`self.machineMaterial`)))