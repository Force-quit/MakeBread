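; BP_Dropper is an actor that spawns a steady series of BP_Bread items in the bread game.
; It drops one on BeginPlay at the DoughDropPoint component's location, at a small fixed scale, and stores it as the last dropped item.
; Each tick, it spawns the next once the horizontal distance between itself and that item reaches DistanceWhenDropNew, so spacing depends on distance instead of a timer.
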(event `self.ReceiveBeginPlay`
  (`self.DropNewItem`)
  (`self.SetActorTickEnabled` true))

(event `self.ReceiveTick`
  (params (DeltaSeconds :type "Float (single-precision)"))
  (bind (_returnvalue_x _returnvalue_y) (`KismetMathLibrary.BreakVector` (- (`self.K2_GetActorLocation`) (`self.K2_GetActorLocation` (`self.lastDroppedItem`)))))
  (if (>= (`KismetMathLibrary.VSize` (`KismetMathLibrary.MakeVector` _returnvalue_x _returnvalue_y)) (`self.distanceWhenDropNew`))
    (`self.DropNewItem`)))

(event `DropNewItem`
  (bind _returnvalue (`|SpawnActorFromClass` "/Game/BreadGame/Blueprint/Breads/BP_Bread.BP_Bread_C" (`KismetMathLibrary.MakeTransform` (`SceneComponent.K2_GetComponentLocation` (`self.DoughDropPoint`)) (struct) (0.12 0.12 0.12)) "Undefined" "OverrideRootScale" null null))
  (set `self.lastDroppedItem` _returnvalue))

(fn `UserConstructionScript`)