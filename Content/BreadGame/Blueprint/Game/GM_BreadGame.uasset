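; Game mode for a bread-making game that holds the bread count and checks for a winning threshold.
; BreadMade adds the multiplier to the count, prints it and calls EndGameCondition at a high threshold, which rechecks a lower one before calling EndGame.
; Spend sets the count to the amount passed minus the current count.
; EndGame is empty, with its QuitGame node left unconnected.
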(event `Spend`
  (params (breadAmount :type Integer))
  ;[1 1 1] Spend
  (set `self.nbBreads` (- breadAmount (`self.nbBreads`))))

(event `BreadMade`
  ;[1 1 1] BreadMade
  (bind _output_get (set `self.nbBreads` (+ (`self.nbBreads`) (`self.breadMult`))))
  (`KismetSystemLibrary.PrintString` (`KismetStringLibrary.Conv_Int64ToString` _output_get))
  (if (>= _output_get 100000)
    (`self.EndGameCondition`)))

(fn `EndGame`)

(fn `EndGameCondition`
  (if (>= (`self.nbBreads`) 1000)
    (`self.EndGame`)))

(fn `UserConstructionScript`)