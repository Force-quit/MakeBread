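; BP_BreadGame is the rule Blueprint for a bread-making game, tracking the bread count and checking for the end condition.
; BeginPlay resets the count and multiplier, shows the mouse cursor and resets move-input ignoring.
; Each OnBreadComplete adds the multiplier, prints the total and calls EndGameCondition from 100000 breads, which rechecks against 1000.
; EndGame is an empty stub, with its QuitGame node left unconnected.
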(event `self.ReceiveBeginPlay`
  (bind _returnvalue (`GameplayStatics.GetPlayerController` 0))
  ;[1 1 1] Initialization
  (set `self.nbBreads` 0)
  (set `self.breadMult` 1)
  (set `PlayerController.bShowMouseCursor` true _returnvalue)
  (`Controller.ResetIgnoreMoveInput` _returnvalue))

(event `OnBreadComplete`
  ;[1 1 1] OnBreadMade
  (bind _output_get (set `self.nbBreads` (+ (`self.nbBreads`) (`self.breadMult`))))
  (`KismetSystemLibrary.PrintString` (`KismetStringLibrary.Conv_Int64ToString` _output_get))
  (if (>= _output_get 100000)
    (`self.EndGameCondition`)))

(fn `EndGame`)

(fn `EndGameCondition`
  (if (>= (`self.nbBreads`) 1000)
    (`self.EndGame`)))

(fn `UserConstructionScript`)